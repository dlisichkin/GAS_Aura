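; Melee attack gameplay ability that turns the avatar toward its combat target and plays an attack montage.
; Activation gets the target from the avatar, updates its facing through CombatInterface, then starts the montage and a melee-hit gameplay event wait.
; The damage effect spec, at ability level, is applied immediately after the wait starts with no target wired; the hit event only draws a debug sphere.
; Montage completion, interruption or cancellation ends the ability.
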(event Ability|EventActivateAbility
  (bind _returnvalue (Ability|GetAvatarActorfromActorInfo))
  (bind _returnvalue_2 (Ability|GetAbilitySystemComponentfromActorInfo))
  (Utilities|IsValid _returnvalue
    (:Is%20Valid
      (bind _output_get (Variables|Default|SetAvatarActor _returnvalue))
      (bind _returnvalue_3 (Class|EnemyInterface|GetCombatTarget(Message) _output_get))
      (Utilities|IsValid _returnvalue_3
        (:Is%20Valid
          (bind _output_get_2 (Variables|Default|SetCombatTarget _returnvalue_3))
          (bind _ascombat_interface (Utilities|Casting|CastToCombatInterface _output_get_2))
          (Class|CombatInterface|UpdateFacingTarget _ascombat_interface (Transformation|GetActorLocation (Variables|Default|GetCombatTarget)))
          (|PlayMontageandWaitProxy "None" (Variables|Default|GetAttackMontage) 1.0 "None" true 1.0 0.0 false
            (:then
              (Ability|Tasks|WaitGameplayEvent "(TagName=\"Event.Monatage.MeleeHit\")" 0
                (:then
                  (GameplayEffects|ApplyGameplayEffectSpecToTarget :EffectSpecHandle (GameplayEffects|MakeOutgoingSpec _returnvalue_2 (Variables|Default|GetDamageEffectClass) (Math|Conversions|ToFloat(Integer) (Ability|GetAbilityLevel)) (GameplayEffects|MakeEffectContext _returnvalue_2))))
                (:EventReceived
                  (Rendering|Debug|DrawDebugSphere (Transformation|GetActorLocation (Ability|GetAvatarActorfromActorInfo)) 1e+02 12 "(R=1.000000,G=0.996646,B=0.047743,A=1.000000)" 0.5))))
            (:OnCompleted
              (Ability|EndAbility :!label _label))
            (:OnInterrupted
              (goto _label))
            (:OnCancelled
              (goto _label))))))))

(event Ability|EventOnEndAbility
  (params (bWasCancelled :type Boolean)))