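; Fire Bolt gameplay ability that spawns a projectile from the Aura player character when activated on the server.
; It reads the combat socket location through the combat interface and spawns the configured projectile class there with zero rotation.
; The owning actor, cast to PlayerState, supplies the projectile's owner and its pawn the instigator.
; EndAbility is called only after a successful spawn, not on the client or failure paths.
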(event Ability|EventActivateAbility
  (bind _returnvalue (Ability|GetOwningActorfromActorInfo))
  (Ability|HasAuthority
    (:True
      (bind _asaura_character (Utilities|Casting|CastToAuraCharacter (Ability|GetAvatarActorfromActorInfo)))
      (if (Utilities|DoesObjectImplementInterface _asaura_character (Variables|Default|GetCombatInterfaceClass))
        (bind _returnvalue_2 (Class|AuraCharacterBase|GetCombatSocketLocation _asaura_character))
        (bind _output_get (Variables|Default|SetSpawnTransform (Math|Transform|MakeTransform _returnvalue_2)))
        (bind _asplayer_state (Utilities|Casting|CastToPlayerState _returnvalue)
          (:then
            (bind _returnvalue_3 (Game|SpawnActorfromClass (Variables|Default|GetProjectileClass) _output_get "AlwaysSpawn" "MultiplyWithRoot" _returnvalue (PlayerState|GetPawn _asplayer_state)))
            (Variables|Default|SetProjectile _returnvalue_3)
            (Ability|EndAbility))
          (:CastFailed
            (Development|PrintString "Cast to Pawn Failed" true true "(R=0.843933,G=0.304575,B=1.000000,A=1.000000)")))))))

(event Ability|EventOnEndAbility
  (params (bWasCancelled :type Boolean)))